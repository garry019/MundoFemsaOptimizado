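; Wellness sign actor (CartelBienestar) that plays a video when something overlaps its Box trigger.
; Begin overlap latently opens the MediaSource on the MediaPlayer and plays it, with a Playing flag blocking retriggers until the VideoTimer delay ends.
; End overlap pauses and rewinds the player but leaves Playing to clear on that timer.
; Neither overlap event filters by actor.
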(event OnComponentBeginOverlap(Box)
  (params (OverlappedComponent :type Primitive%20Component%20Object%20Reference) (OtherActor :type Actor%20Object%20Reference) (OtherComp :type Primitive%20Component%20Object%20Reference) (OtherBodyIndex :type Integer) (bFromSweep :type Boolean) (SweepResult :type Hit%20Result%20Structure%20%28by%20ref%29))
  (bind _mediaplayer (Variables|Default|GetMediaPlayer))
  (if (not (Variables|Default|GetPlaying))
    (Variables|Default|SetPlaying true)
    (Class|MediaPlayer|OpenSourceLatent _mediaplayer (Variables|Default|GetMedia%20Source))
    (Media|MediaPlayer|Play _mediaplayer :!class /Script/MediaAssets.MediaPlayer)
    (Utilities|FlowControl|Delay (Variables|Default|GetVideoTimer))
    (Variables|Default|SetPlaying false)))

(event OnComponentEndOverlap(Box)
  (params (OverlappedComponent :type Primitive%20Component%20Object%20Reference) (OtherActor :type Actor%20Object%20Reference) (OtherComp :type Primitive%20Component%20Object%20Reference) (OtherBodyIndex :type Integer))
  (bind _mediaplayer (Variables|Default|GetMediaPlayer))
  (Sequencer|Player|Pause _mediaplayer)
  (Class|MediaPlayer|Rewind _mediaplayer))

(fn ConstructionScript)