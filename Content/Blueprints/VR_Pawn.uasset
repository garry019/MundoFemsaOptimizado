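; VR player pawn with floor-level tracking, object grabbing, thumbstick turning and navmesh-validated teleportation.
; Each grip sends hold and drop messages to the first BP_Interactive_Object overlapping that hand's collision.
; Left stick X applies gated one-shot yaw steps that re-arm inside the dead zone.
; Pushing right stick Y traces a projectile arc to place a teleport marker; releasing it moves the pawn after a delay, and X cancels.
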(event EventBeginPlay
  (Class|HeadMountedDisplayFunctionLibrary|SetTrackingOrigin "Floor"))

(event Input|ActionEvents|InputActionMotionController_XPress
  (params (Key :type Key%20Structure :default "None"))
  (:Pressed
    (Variables|Default|SetCancelTeleport true)
    (if (Variables|Default|GetTeleportMakActive)
      (Actor|DestroyActor (Variables|Default|GetTeleportMark))
      (Variables|Default|SetTraceActive false)
      (Variables|Default|SetTeleportMakActive false))))

(event Input|ActionEvents|InputActionMotionController_Right_Grip
  (params (Key :type Key%20Structure :default "None"))
  (bind _collitionright (Variables|Default|GetCollitionRight))
  (bind _mc_right (Variables|Default|GetMC_Right))
  (bind _overlappingactors (Collision|GetOverlappingActors _collitionright "/Game/Interaction/BP_Interactive_Object.BP_Interactive_Object_C" :!class /Script/Engine.PrimitiveComponent))
  (bind _output (Utilities|Array|Get(acopy) _overlappingactors))
  ;[1 1 1] Grip Mano derecha
  (:Pressed
    (Class|BPInteractionInterface|HoldObject(Message) _output _mc_right)
    (bind _output_get (Variables|Default|SetObjectHoldByRight true)))
  (:Released
    (if _output_get
      (Class|BPInteractionInterface|DropObject(Message) _output _mc_right)
      (Variables|Default|SetObjectHoldByRight false))))

(event Input|ActionEvents|InputActionMotionController_Left_Grip
  (params (Key :type Key%20Structure :default "None"))
  (bind _mc_left (Variables|Default|GetMC_Left))
  (bind _collitionleft (Variables|Default|GetCollitionLeft))
  (bind _overlappingactors (Collision|GetOverlappingActors _collitionleft "/Game/Interaction/BP_Interactive_Object.BP_Interactive_Object_C" :!class /Script/Engine.PrimitiveComponent))
  (bind _output (Utilities|Array|Get(acopy) _overlappingactors))
  ;[1 1 1] Grip Mano Izquierda
  (:Pressed
    (Class|BPInteractionInterface|HoldObject(Message) _output _mc_left)
    (bind _output_get (Variables|Default|SetObjectHoldByLeft true)))
  (:Released
    (if _output_get
      (Class|BPInteractionInterface|DropObject(Message) _output _mc_left)
      (Variables|Default|SetObjectHoldByLeft false))))

(event Input|AxisEvents|InputAxisLeft_Thumbstick_X
  (params (AxisValue :type Float%20%28single-precision%29))
  (bind _turnvalue (Variables|Default|GetTurnValue))
  ;[1 1 1] Girar personaje
  (if (>= (Math|Float|Absolute(Float) AxisValue) (Variables|Default|GetDeadZoneTresHold))
    (if (>= AxisValue 0.0)
      (|DoOnceMultiInput :!label _label
        (:A%20Out
          (Pawn|Input|AddControllerYawInput _turnvalue)))
      (else
        (|DoOnceMultiInput :!label _label_2
          (:A%20Out
            (Pawn|Input|AddControllerYawInput (* _turnvalue -1.0))))))
    (else
      (Utilities|FlowControl|MultiGate false true -1
        (:Out%200
          (goto _label Reset%20In))
        (:Out%201
          (goto _label_2 Reset%20In))))))

(event Input|AxisEvents|InputAxisRight_Thumbstick_Y
  (params (AxisValue :type Float%20%28single-precision%29))
  (bind _mc_right (Variables|Default|GetMC_Right))
  (if (>= AxisValue (Variables|Default|GetDeadZoneTresHold))
    (if (not (Variables|Default|GetCancelTeleport))
      (Utilities|FlowControl|Sequence
        (:then_0
          (CallFunction|TeleportTrace (Transformation|GetWorldLocation _mc_right) (Math|Vector|GetForwardVector _mc_right))
          (Variables|Default|SetTraceActive true))))
    (else
      (Variables|Default|SetCancelTeleport false)
      (if (and (Variables|Default|GetTraceActive) (Variables|Default|GetValidTeleportLocation))
        (Actor|DestroyActor (Variables|Default|GetTeleportMark))
        (Variables|Default|SetTraceActive false)
        (Variables|Default|SetTeleportMakActive false)
        (Utilities|FlowControl|Delay 0.45)
        (Transformation|SetActorLocation (Variables|Default|GetTeleportLocation) false false)
        (Variables|Default|SetCancelTeleport false)))))

(fn ConstructionScript)

(fn TeleportTrace
  (params (CutrrentLocation :type Vector) (ForwardVector :type Vector))
  (bind _outactors (Actor|GetAllActorsOfClass "/Game/Interaction/BP_Interactive_Object.BP_Interactive_Object_C"))
  (bind (_outhit _outpathpositions _outlasttracedestination) (Class|GameplayStatics|BlueprintPredictProjectilePathbyTraceChannel CutrrentLocation (* ForwardVector (Variables|Default|GetForwardForce)) true 0.0 "ECC_WorldStatic" false _outactors "ForDuration"))
  (Utilities|FlowControl|Sequence
    (:then_0
      (Utilities|FlowControl|DoOnce (Variables|Default|GetTeleportMakActive)
        (:Completed
          (bind _returnvalue (Game|SpawnActorfromClass "/Game/Blueprints/BP_TeleportMark.BP_TeleportMark_C" (Math|Transform|MakeTransform _outlasttracedestination "0, 0, 0" "0.500000,0.500000,0.100000") "Undefined" 0 0))
          (bind _output_get (Variables|Default|SetTeleportMark _returnvalue))
          (Variables|Default|SetTeleportMakActive true))))
    (:then_1
      (Transformation|SetRelativeLocation (Variables|/Game/Blueprints/BP_TeleportMark.BP_TeleportMark_C|GetCylinder _output_get) (.ProjectedLocation (AI|Navigation|ProjectPointtoNavigation _outlasttracedestination 0 0 "0, 0, 0")) false false)
      (Variables|Default|SetTeleportLocation (.ProjectedLocation (AI|Navigation|ProjectPointtoNavigation _outlasttracedestination 0 0 "0, 0, 0"))))
    (:then_2
      (Variables|Default|SetValidTeleportLocation (.ReturnValue (AI|Navigation|ProjectPointtoNavigation (Class|NavigationSystemV1|GetNavigationSystem) (.Location (Collision|BreakHitResult _outhit)) 0 0))))))