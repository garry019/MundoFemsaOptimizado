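; VR player character with stick movement, snap turning, grip hold/drop of interactive objects and trigger clicks on widgets.
; BeginPlay restores location from BP_GameInstances, spawning a Niagara pointer laser for debug or the final view, which also reveals BPFinal.
; Otherwise, intro audio starts, and chained events switch media players while revealing each instruction panel.
; Tick blocks movement during intro and final view by inflating the stick deadzone.
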(event Custom|SpawnLaser
  ;[1 1 1] Laser Beam - Visual interaction
  (bind _returnvalue (Niagara|SpawnSystemAttached "/Game/Widgets/VFX/NS_Pointer.NS_Pointer" (Variables|Default|GetSM_Right) "Pointer" "0, 0, 0" "0, 0, 0" "SnapToTarget" false))
  (Variables|Default|SetLaserSpawned _returnvalue))

(event Custom|Introduccion_1
  (bind _mediaplayer_intro1 (Variables|Default|GetMediaPlayer_Intro1))
  (Sequencer|Player|Pause (Variables|Default|GetMediaPlayer))
  (bind _asbp_game_instances (Utilities|Casting|CastToBP_GameInstances (Game|GetGameInstance)))
  (if (Variables|/Game/Blueprints/BP_GameInstances.BP_GameInstances_C|GetIntroWidget _asbp_game_instances)
    (bind _output_get (Variables|Default|SetPlaying true))
    (if _output_get
      (Class|MediaPlayer|OpenSourceLatent _mediaplayer_intro1 (Variables|Default|GetMedia%20Source_Intro1))
      (Media|MediaPlayer|Play _mediaplayer_intro1 :!class /Script/MediaAssets.MediaPlayer)
      (bind _returnvalue (Actor|GetActorOfClass "/Game/Widgets/Instrucciones/BP_Instrucciones.BP_Instrucciones_C"))
      (Rendering|SetVisibility (Variables|/Game/Widgets/Instrucciones/BP_Instrucciones.BP_Instrucciones_C|GetfemsaVRButton _returnvalue) true false)
      (Rendering|SetVisibility (Variables|/Game/Widgets/Instrucciones/BP_Instrucciones.BP_Instrucciones_C|GetText3D _returnvalue) true false)
      (Rendering|SetVisibility (Variables|/Game/Widgets/Instrucciones/BP_Instrucciones.BP_Instrucciones_C|GetWidget _returnvalue) true false))))

(event Custom|Instrucciones_3
  (bind _mediaplayer_instrucciones3 (Variables|Default|GetMediaPlayer_Instrucciones3))
  (Sequencer|Player|Pause (Variables|Default|GetMediaPlayer_Instrucciones2))
  (bind _asbp_game_instances (Utilities|Casting|CastToBP_GameInstances (Game|GetGameInstance)))
  (if (Variables|/Game/Blueprints/BP_GameInstances.BP_GameInstances_C|GetIntroWidget _asbp_game_instances)
    (bind _output_get (Variables|Default|SetPlaying true))
    (if _output_get
      (Class|MediaPlayer|OpenSourceLatent _mediaplayer_instrucciones3 (Variables|Default|GetMedia%20Source_Instrucciones3))
      (Media|MediaPlayer|Play _mediaplayer_instrucciones3 :!class /Script/MediaAssets.MediaPlayer)
      (bind _returnvalue (Actor|GetActorOfClass "/Game/Widgets/Instrucciones/BP_Instrucciones_5.BP_Instrucciones_5_C"))
      (Rendering|SetVisibility (Variables|/Game/Widgets/Instrucciones/BP_Instrucciones_5.BP_Instrucciones_5_C|GetfemsaVRButton _returnvalue) true false)
      (Rendering|SetVisibility (Variables|/Game/Widgets/Instrucciones/BP_Instrucciones_5.BP_Instrucciones_5_C|GetText3D _returnvalue) true false)
      (Rendering|SetVisibility (Variables|/Game/Widgets/Instrucciones/BP_Instrucciones_5.BP_Instrucciones_5_C|GetWidget _returnvalue) true false))))

(event Custom|Instrucciones_4
  (bind _mediaplayer_instrucciones4 (Variables|Default|GetMediaPlayer_Instrucciones4))
  (Sequencer|Player|Pause (Variables|Default|GetMediaPlayer_Instrucciones3))
  (bind _asbp_game_instances (Utilities|Casting|CastToBP_GameInstances (Game|GetGameInstance)))
  (if (Variables|/Game/Blueprints/BP_GameInstances.BP_GameInstances_C|GetIntroWidget _asbp_game_instances)
    (bind _output_get (Variables|Default|SetPlaying true))
    (if _output_get
      (Class|MediaPlayer|OpenSourceLatent _mediaplayer_instrucciones4 (Variables|Default|GetMedia%20Source_Instrucciones4))
      (Media|MediaPlayer|Play _mediaplayer_instrucciones4 :!class /Script/MediaAssets.MediaPlayer)
      (bind _returnvalue (Actor|GetActorOfClass "/Game/Widgets/Instrucciones/BP_Instrucciones_6.BP_Instrucciones_6_C"))
      (Rendering|SetVisibility (Variables|/Game/Widgets/Instrucciones/BP_Instrucciones_6.BP_Instrucciones_6_C|GetfemsaVRButton _returnvalue) true false)
      (Rendering|SetVisibility (Variables|/Game/Widgets/Instrucciones/BP_Instrucciones_6.BP_Instrucciones_6_C|GetText3D _returnvalue) true false)
      (Rendering|SetVisibility (Variables|/Game/Widgets/Instrucciones/BP_Instrucciones_6.BP_Instrucciones_6_C|GetWidget _returnvalue) true false))))

(event Custom|DestroyPointer
  (bind _laserspawned (Variables|Default|GetLaserSpawned))
  ;[1 1 1] Laser Beam - Visual interaction
  (Utilities|IsValid _laserspawned
    (:Is%20Valid
      (Rendering|SetVisibility _laserspawned false false))))

(event Custom|Introduccion_2
  (bind _mediaplayer_intro2 (Variables|Default|GetMediaPlayer_Intro2))
  (Sequencer|Player|Pause (Variables|Default|GetMediaPlayer_Intro1))
  (bind _asbp_game_instances (Utilities|Casting|CastToBP_GameInstances (Game|GetGameInstance)))
  (if (Variables|/Game/Blueprints/BP_GameInstances.BP_GameInstances_C|GetIntroWidget _asbp_game_instances)
    (bind _output_get (Variables|Default|SetPlaying true))
    (if _output_get
      (Class|MediaPlayer|OpenSourceLatent _mediaplayer_intro2 (Variables|Default|GetMedia%20Source_Intro2))
      (Media|MediaPlayer|Play _mediaplayer_intro2 :!class /Script/MediaAssets.MediaPlayer)
      (bind _returnvalue (Actor|GetActorOfClass "/Game/Widgets/Instrucciones/BP_Instrucciones_2.BP_Instrucciones_2_C"))
      (Rendering|SetVisibility (Variables|/Game/Widgets/Instrucciones/BP_Instrucciones_2.BP_Instrucciones_2_C|GetfemsaVRButton _returnvalue) true false)
      (Rendering|SetVisibility (Variables|/Game/Widgets/Instrucciones/BP_Instrucciones_2.BP_Instrucciones_2_C|GetText3D _returnvalue) true false)
      (Rendering|SetVisibility (Variables|/Game/Widgets/Instrucciones/BP_Instrucciones_2.BP_Instrucciones_2_C|GetWidget _returnvalue) true false))))

(event Custom|UpdateDistance
  (bind _laserspawned (Variables|Default|GetLaserSpawned))
  (bind _widgetinteractionright (Variables|Default|GetWidgetInteractionRight))
  ;[1 1 1] Laser Beam - Visual interaction
  (Utilities|IsValid _laserspawned
    (:Is%20Valid
      (if (Class|WidgetInteractionComponent|IsOverHitTestVisibleWidget _widgetinteractionright)
        (Niagara|SetNiagaraVariable(Vector3) _laserspawned "BeamEnd" (Math|Vector|MakeVector (.Distance (Collision|BreakHitResult (Class|WidgetInteractionComponent|GetLastHitResult _widgetinteractionright))) 0.0 0.0))
        (else
          (Niagara|SetNiagaraVariable(Vector3) _laserspawned "BeamEnd" (Math|Vector|MakeVector 3e+01 0.0 0.0)))))))

(event Custom|Instrucciones_5
  (bind _mediaplayer_instrucciones5 (Variables|Default|GetMediaPlayer_Instrucciones5))
  (Sequencer|Player|Pause (Variables|Default|GetMediaPlayer_Instrucciones4))
  (bind _asbp_game_instances (Utilities|Casting|CastToBP_GameInstances (Game|GetGameInstance)))
  (if (Variables|/Game/Blueprints/BP_GameInstances.BP_GameInstances_C|GetIntroWidget _asbp_game_instances)
    (bind _output_get (Variables|Default|SetPlaying true))
    (if _output_get
      (Class|MediaPlayer|OpenSourceLatent _mediaplayer_instrucciones5 (Variables|Default|GetMedia%20Source_Instrucciones5))
      (Media|MediaPlayer|Play _mediaplayer_instrucciones5 :!class /Script/MediaAssets.MediaPlayer)
      (bind _returnvalue (Actor|GetActorOfClass "/Game/Widgets/Instrucciones/BP_Instrucciones_7.BP_Instrucciones_7_C"))
      (Rendering|SetVisibility (Variables|/Game/Widgets/Instrucciones/BP_Instrucciones_7.BP_Instrucciones_7_C|GetfemsaVRButton _returnvalue) true false)
      (Rendering|SetVisibility (Variables|/Game/Widgets/Instrucciones/BP_Instrucciones_7.BP_Instrucciones_7_C|GetText3D _returnvalue) true false)
      (Rendering|SetVisibility (Variables|/Game/Widgets/Instrucciones/BP_Instrucciones_7.BP_Instrucciones_7_C|GetWidget _returnvalue) true false))))

(event Custom|Instrucciones_1
  (bind _mediaplayer_instrucciones1 (Variables|Default|GetMediaPlayer_Instrucciones1))
  (Sequencer|Player|Pause (Variables|Default|GetMediaPlayer_Intro2))
  (bind _asbp_game_instances (Utilities|Casting|CastToBP_GameInstances (Game|GetGameInstance)))
  (if (Variables|/Game/Blueprints/BP_GameInstances.BP_GameInstances_C|GetIntroWidget _asbp_game_instances)
    (bind _output_get (Variables|Default|SetPlaying true))
    (if _output_get
      (Class|MediaPlayer|OpenSourceLatent _mediaplayer_instrucciones1 (Variables|Default|GetMedia%20Source_Instrucciones1))
      (Media|MediaPlayer|Play _mediaplayer_instrucciones1 :!class /Script/MediaAssets.MediaPlayer)
      (bind _returnvalue (Actor|GetActorOfClass "/Game/Widgets/Instrucciones/BP_Instrucciones_3.BP_Instrucciones_3_C"))
      (Rendering|SetVisibility (Variables|/Game/Widgets/Instrucciones/BP_Instrucciones_3.BP_Instrucciones_3_C|GetfemsaVRButton _returnvalue) true false)
      (Rendering|SetVisibility (Variables|/Game/Widgets/Instrucciones/BP_Instrucciones_3.BP_Instrucciones_3_C|GetText3D _returnvalue) true false)
      (Rendering|SetVisibility (Variables|/Game/Widgets/Instrucciones/BP_Instrucciones_3.BP_Instrucciones_3_C|GetWidget _returnvalue) true false))))

(event Custom|Instrucciones_2
  (bind _mediaplayer_instrucciones2 (Variables|Default|GetMediaPlayer_Instrucciones2))
  (Sequencer|Player|Pause (Variables|Default|GetMediaPlayer_Instrucciones1))
  (bind _asbp_game_instances (Utilities|Casting|CastToBP_GameInstances (Game|GetGameInstance)))
  (if (Variables|/Game/Blueprints/BP_GameInstances.BP_GameInstances_C|GetIntroWidget _asbp_game_instances)
    (bind _output_get (Variables|Default|SetPlaying true))
    (if _output_get
      (Class|MediaPlayer|OpenSourceLatent _mediaplayer_instrucciones2 (Variables|Default|GetMedia%20Source_Instrucciones2))
      (Media|MediaPlayer|Play _mediaplayer_instrucciones2 :!class /Script/MediaAssets.MediaPlayer)
      (bind _returnvalue (Actor|GetActorOfClass "/Game/Widgets/Instrucciones/BP_Instrucciones_4.BP_Instrucciones_4_C"))
      (Rendering|SetVisibility (Variables|/Game/Widgets/Instrucciones/BP_Instrucciones_4.BP_Instrucciones_4_C|GetfemsaVRButton _returnvalue) true false)
      (Rendering|SetVisibility (Variables|/Game/Widgets/Instrucciones/BP_Instrucciones_4.BP_Instrucciones_4_C|GetText3D _returnvalue) true false)
      (Rendering|SetVisibility (Variables|/Game/Widgets/Instrucciones/BP_Instrucciones_4.BP_Instrucciones_4_C|GetWidget _returnvalue) true false))))

(event EventBeginPlay
  (bind _bp_final (Variables|Default|GetBP_Final))
  (bind _mediaplayer (Variables|Default|GetMediaPlayer))
  (bind _asbp_game_instances (Utilities|Casting|CastToBP_GameInstances (Game|GetGameInstance)))
  (if (Variables|/Game/Blueprints/BP_GameInstances.BP_GameInstances_C|GetShowDebug _asbp_game_instances)
    (CallFunction|SpawnLaser)
    (Utilities|Time|SetTimerbyEvent (EventDispatchers|CreateEvent :!event Custom|UpdateDistance) 0.1 true))
  (Class|HeadMountedDisplayFunctionLibrary|SetTrackingOrigin "Eye")
  (bind _asbp_game_instances_2 (Utilities|Casting|CastToBP_GameInstances (Game|GetGameInstance)))
  (Transformation|SetActorLocation self (Variables|/Game/Blueprints/BP_GameInstances.BP_GameInstances_C|GetCurrentLocation _asbp_game_instances_2) false false)
  (if (Variables|/Game/Blueprints/BP_GameInstances.BP_GameInstances_C|GetLastView _asbp_game_instances_2)
    (Pawn|Input|AddControllerYawInput 3e+01)
    (bind _asbp_game_instances_3 (Utilities|Casting|CastToBP_GameInstances (Game|GetGameInstance)))
    (Variables|/Game/Blueprints/BP_GameInstances.BP_GameInstances_C|SetShowDebug _asbp_game_instances_3 true)
    (CallFunction|SpawnLaser)
    (Utilities|Time|SetTimerbyEvent (EventDispatchers|CreateEvent :!event Custom|UpdateDistance) 0.1 true)
    (Rendering|SetVisibility _bp_final true false)
    (Transformation|SetRelativeScale3D _bp_final "1.000000,1.000000,1.000000")
    (else
      ;[1 1 1] AUDIO INTRO
      (bind _asbp_game_instances_4 (Utilities|Casting|CastToBP_GameInstances (Game|GetGameInstance)))
      (if (Variables|/Game/Blueprints/BP_GameInstances.BP_GameInstances_C|GetIntroWidget _asbp_game_instances_4)
        (bind _output_get (Variables|Default|SetPlaying true))
        (if _output_get
          (Class|MediaPlayer|OpenSourceLatent _mediaplayer (Variables|Default|GetMedia%20Source))
          (Media|MediaPlayer|Play _mediaplayer :!class /Script/MediaAssets.MediaPlayer)
          (bind _returnvalue (Actor|GetActorOfClass "/Game/Widgets/Intro/BP_Intro.BP_Intro_C"))
          (Rendering|SetVisibility (Variables|/Game/Widgets/Intro/BP_Intro.BP_Intro_C|GetfemsaVRButton _returnvalue) true false)
          (Rendering|SetVisibility (Variables|/Game/Widgets/Intro/BP_Intro.BP_Intro_C|GetText3D1 _returnvalue) true false)
          (Rendering|SetVisibility (Variables|/Game/Widgets/Intro/BP_Intro.BP_Intro_C|GetWidget _returnvalue) true false))))))

(event EventTick
  (params (DeltaSeconds :type Float%20%28single-precision%29))
  (bind _self self)
  (bind _asbp_game_instances (Utilities|Casting|CastToBP_GameInstances (Game|GetGameInstance)))
  (Variables|/Script/UMG.WidgetInteractionComponent|SetbShowDebug (Variables|Default|GetWidgetInteractionRight) (Variables|/Game/Blueprints/BP_GameInstances.BP_GameInstances_C|GetShowDebug _asbp_game_instances))
  (if (and (Variables|/Game/Blueprints/BP_GameInstances.BP_GameInstances_C|GetIntroWidget _asbp_game_instances) (Variables|Default|GetIntroWidgetVisible))
    (Variables|VR_Character_C|SetMovementDeadzone self 5e+02))
  (if (Variables|/Game/Blueprints/BP_GameInstances.BP_GameInstances_C|GetLastView (stale EventBeginPlay _asbp_game_instances_2))
    (Variables|VR_Character_C|SetMovementDeadzone _self 5e+02)
    (elif (Variables|Default|GetIntroWidgetVisible)
      (Variables|VR_Character_C|SetMovementDeadzone _self 5e+02)
      (else
        (Variables|VR_Character_C|SetMovementDeadzone _self 0.8)))))

(event Input|ActionEvents|InputActionMotionController_Right_Trigger
  (params (Key :type Key%20Structure :default "None"))
  (bind _widgetinteractionright (Variables|Default|GetWidgetInteractionRight))
  (:Pressed
    (Class|WidgetInteractionComponent|PressPointerKey _widgetinteractionright "LeftMouseButton"))
  (:Released
    (Class|WidgetInteractionComponent|ReleasePointerKey _widgetinteractionright "LeftMouseButton")))

(event Input|ActionEvents|InputActionMotionController_Right_Grip
  (params (Key :type Key%20Structure :default "None"))
  (bind _collitionright (Variables|Default|GetCollitionRight))
  (bind _mc_right (Variables|Default|GetMC_Right))
  (bind _overlappingactors (Collision|GetOverlappingActors _collitionright "/Game/Interaction/BP_Interactive_Object.BP_Interactive_Object_C" :!class /Script/Engine.PrimitiveComponent))
  (bind _output (Utilities|Array|Get(acopy) _overlappingactors))
  ;[1 1 1] Grip Mano derecha
  (:Pressed
    (Class|BPInteractionInterface|HoldObject(Message) _output _mc_right)
    (bind _output_get (Variables|Default|SetObjectHoldByRight true)))
  (:Released
    (if _output_get
      (Class|BPInteractionInterface|DropObject(Message) _output _mc_right)
      (Variables|Default|SetObjectHoldByRight false))))

(event Input|ActionEvents|InputActionMotionController_Left_Grip
  (params (Key :type Key%20Structure :default "None"))
  (bind _mc_left (Variables|Default|GetMC_Left))
  (bind _collitionleft (Variables|Default|GetCollitionLeft))
  (bind _overlappingactors (Collision|GetOverlappingActors _collitionleft "/Game/Interaction/BP_Interactive_Object.BP_Interactive_Object_C" :!class /Script/Engine.PrimitiveComponent))
  (bind _output (Utilities|Array|Get(acopy) _overlappingactors))
  ;[1 1 1] Grip Mano Izquierda
  (:Pressed
    (Class|BPInteractionInterface|HoldObject(Message) _output _mc_left)
    (bind _output_get (Variables|Default|SetObjectHoldByLeft true)))
  (:Released
    (if _output_get
      (Class|BPInteractionInterface|DropObject(Message) _output _mc_left)
      (Variables|Default|SetObjectHoldByLeft false))))

(event Input|AxisEvents|InputAxisLeft_Thumbstick_X
  (params (AxisValue :type Float%20%28single-precision%29))
  (bind _turnvalue (Variables|Default|GetTurnValue))
  ;[1 1 1] Girar personaje
  (if (>= (Math|Float|Absolute(Float) AxisValue) (Variables|Default|GetDeadZoneTresHold))
    (if (>= AxisValue 0.0)
      (|DoOnceMultiInput :!label _label
        (:A%20Out
          (Pawn|Input|AddControllerYawInput _turnvalue)))
      (else
        (|DoOnceMultiInput :!label _label_2
          (:A%20Out
            (Pawn|Input|AddControllerYawInput (* _turnvalue -1.0))))))
    (else
      (Utilities|FlowControl|MultiGate false true -1
        (:Out%200
          (goto _label Reset%20In))
        (:Out%201
          (goto _label_2 Reset%20In))))))

(event Input|AxisEvents|InputAxisRight_Thumbstick_X
  (params (AxisValue :type Float%20%28single-precision%29))
  (if (>= (Math|Float|Absolute(Float) AxisValue) (Variables|Default|GetMovementDeadzone))
    (Pawn|Input|AddMovementInput (Math|Vector|GetRightVector (Variables|Default|GetCamera)) (* AxisValue (Variables|Default|GetMovementScalar)) false)))

(event Input|AxisEvents|InputAxisRight_Thumbstick_Y
  (params (AxisValue :type Float%20%28single-precision%29))
  (if (>= (Math|Float|Absolute(Float) AxisValue) (Variables|Default|GetMovementDeadzone))
    (Pawn|Input|AddMovementInput (Math|Vector|GetForwardVector (Variables|Default|GetCamera)) (* AxisValue (Variables|Default|GetMovementScalar)) false)))

(fn ConstructionScript)