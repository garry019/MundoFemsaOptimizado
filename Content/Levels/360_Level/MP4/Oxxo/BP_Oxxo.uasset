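; BP_Oxxo runs the Oxxo 360 video level in VR, then returns the player to DEMO_Map.
; On BeginPlay it fades via WB_MapTeleport, stores a hardcoded return location and rotation in the game instance, shows hand widgets, spawns a laser and plays the media.
; After a VideoTimer delay it fades, removes the pointer and opens the map.
; An unconnected variant times the exit from the media's duration instead.
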(event EventBeginPlay
  (bind _mediaplayer (Variables|Default|GetMediaPlayer))
  (bind _returnvalue (UserInterface|CreateWidget "/Game/Levels/360_Level/Teleport/WB_MapTeleport.WB_MapTeleport_C"))
  (UserInterface|Viewport|AddtoViewport _returnvalue 0)
  (Default|FadeOutAnimation _returnvalue)
  (Utilities|FlowControl|Delay 0.5)
  (bind _asbp_game_instances (Utilities|Casting|CastToBP_GameInstances (Game|GetGameInstance)))
  (Variables|/Game/Blueprints/BP_GameInstances.BP_GameInstances_C|SetCurrentLocation _asbp_game_instances "10595.412109,1802.352295,1970.124756")
  (Variables|/Game/Blueprints/BP_GameInstances.BP_GameInstances_C|SetRotation _asbp_game_instances "0.000000, 0,100.000000")
  (bind _returnvalue_2 (Actor|GetActorOfClass "/Game/Blueprints/VR_Character.VR_Character_C"))
  (Rendering|SetVisibility (Variables|/Game/Blueprints/VR_Character.VR_Character_C|GetHandWidget _returnvalue_2) true false)
  (Rendering|SetVisibility (Variables|/Game/Blueprints/VR_Character.VR_Character_C|GetBP_HandWidget _returnvalue_2) true false)
  (Variables|/Game/Blueprints/BP_GameInstances.BP_GameInstances_C|SetShowDebug _asbp_game_instances true)
  (Default|SpawnLaser _returnvalue_2)
  (Class|MediaPlayer|OpenSourceLatent _mediaplayer (Variables|Default|GetMedia%20Source))
  (Media|MediaPlayer|Play _mediaplayer :!class /Script/MediaAssets.MediaPlayer)
  (Utilities|FlowControl|Delay (Variables|Default|GetVideoTimer))
  (bind _returnvalue_3 (UserInterface|CreateWidget "/Game/Levels/360_Level/Teleport/WB_MapTeleport.WB_MapTeleport_C"))
  (UserInterface|Viewport|AddtoViewport _returnvalue_3 0)
  (Default|FadeAnimation _returnvalue_3)
  (Variables|/Game/Blueprints/BP_GameInstances.BP_GameInstances_C|SetShowDebug _asbp_game_instances false)
  (Default|DestroyPointer _returnvalue_2)
  (Utilities|FlowControl|Delay 0.5)
  (Game|OpenLevel(byName) "DEMO_Map"))

(fn ConstructionScript)